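; Player controller for a Pong game that handles per-level UI, score tracking and the end of a match.
; BeginPlay adds the menu, Pong HUD or credits widget based on level name, and caches the Ball_BP actor in Map_01.
; In that map, Tick polls the ball's counters, converts them to score text and checks both against the cap.
; On a win, it saves scores and winner to the GameOver slot, then opens Credits.
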(event Custom|Creditos
  ;[1 1 1] Savegame variables
  (bind _returnvalue (SaveGame|CreateSaveGameObject "/Game/Blueprints/SaveGamePong.SaveGamePong_C"))
  ;;[1 1 1] Saves Variables to gameslot
  (Variables|Default|Setgamesave _returnvalue)
  (Variables|/Game/Blueprints/SaveGamePong.SaveGamePong_C|Setp1 (Variables|Default|Getgamesave) (Variables|Default|GetScore_P1))
  (Variables|/Game/Blueprints/SaveGamePong.SaveGamePong_C|Setp2 (Variables|Default|Getgamesave) (Variables|Default|GetScore_P2))
  (Variables|/Game/Blueprints/SaveGamePong.SaveGamePong_C|SetWin (Variables|Default|Getgamesave) (Variables|Default|GetWinner))
  (SaveGame|SaveGametoSlot (Variables|Default|Getgamesave) "GameOver")
  (Game|OpenLevel(byName) "Credits"))

(event EventBeginPlay
  ;[1 1 1] On BeginPlay (Run Once)
  ;;[1 1 1] Check if Menu
  (bind _returnvalue (Game|GetCurrentLevelName true))
  (if (Utilities|Enum|Equal(Enum) _returnvalue "Menu")
    ;;[1 1 1] Create Menu Widget
    (bind _returnvalue_2 (UserInterface|CreateWidget "/Game/Blueprints/MenuWidget.MenuWidget_C" self)) ; Create the Widget
    (UserInterface|Viewport|AddtoViewport _returnvalue_2 0) ; Make it Viewable
    (else
      ;;[1 1 1] Check if Main Map
      (bind _returnvalue_3 (Game|GetCurrentLevelName true))
      (if (Utilities|Enum|Equal(Enum) _returnvalue_3 "Map_01")
        ;;[1 1 1] Create Main map widget
        (bind _returnvalue_4 (UserInterface|CreateWidget "/Game/Blueprints/PongWidget.PongWidget_C" self)) ; Create the Widget
        (UserInterface|Viewport|AddtoViewport _returnvalue_4 0) ; Make it Viewable
        ;;[1 1 1] Get the Actors of the Actor BluePrint
        (bind _outactors (Actor|GetAllActorsOfClass "/Game/Blueprints/Ball_BP.Ball_BP_C"))
        (Variables|Default|SetBall (Utilities|Array|Get(acopy) _outactors)) ; Set the Actor instance to a usable Actor Copy
        (else
          ;;[1 1 1] If its not Menu or Main Map its credits
          (bind _returnvalue_5 (UserInterface|CreateWidget "/Game/Blueprints/CreditWidget.CreditWidget_C" self)) ; Create the Widget
          (UserInterface|Viewport|AddtoViewport _returnvalue_5 0) ; Make it Viewable
        )))))

(event EventTick
  (params (DeltaSeconds :type Float%20%28single-precision%29))
  ;[1 1 1] Points and Map pass
  ;;[1 1 1] Checks Map name
  (bind _returnvalue (Game|GetCurrentLevelName true))
  (if (Utilities|Enum|Equal(Enum) _returnvalue "Map_01")
    ;;[1 1 1] Winner Check + Score Set per tick
    (if (== (Variables|Default|GetCap_Score) (Variables|/Game/Blueprints/Ball_BP.Ball_BP_C|Getcounter_P1 (Variables|Default|GetBall)))
      (Variables|Default|SetScore_P1 (Utilities|Text|ToText(Integer) (Variables|/Game/Blueprints/Ball_BP.Ball_BP_C|Getcounter_P1 (Variables|Default|GetBall))))
      (Variables|Default|SetScore_P2 (Utilities|Text|ToText(Integer) (Variables|/Game/Blueprints/Ball_BP.Ball_BP_C|Getcounter_P2 (Variables|Default|GetBall))))
      ;;[1 1 1] Saves Winner
      (Variables|Default|SetWin_P1 true)
      (Variables|Default|SetWinner "1")
      ;;[1 1 1] Triggers the Savegame event
      (CallFunction|Creditos self :!label _label)
      (elif (== (Variables|/Game/Blueprints/Ball_BP.Ball_BP_C|Getcounter_P2 (Variables|Default|GetBall)) (Variables|Default|GetCap_Score))
        (Variables|Default|SetScore_P1 (Utilities|Text|ToText(Integer) (Variables|/Game/Blueprints/Ball_BP.Ball_BP_C|Getcounter_P1 (Variables|Default|GetBall))))
        (Variables|Default|SetScore_P2 (Utilities|Text|ToText(Integer) (Variables|/Game/Blueprints/Ball_BP.Ball_BP_C|Getcounter_P2 (Variables|Default|GetBall))))
        (Variables|Default|SetWin_P2 true)
        (Variables|Default|SetWinner "2")
        (goto _label)
        (else
          (Variables|Default|SetScore_P1 (Utilities|Text|ToText(Integer) (Variables|/Game/Blueprints/Ball_BP.Ball_BP_C|Getcounter_P1 (Variables|Default|GetBall))))
          (Variables|Default|SetScore_P2 (Utilities|Text|ToText(Integer) (Variables|/Game/Blueprints/Ball_BP.Ball_BP_C|Getcounter_P2 (Variables|Default|GetBall)))))))))

(fn ConstructionScript)