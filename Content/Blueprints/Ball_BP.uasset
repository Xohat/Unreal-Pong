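; Pong ball Blueprint that moves a physics sphere, bounces it and counts goals for both players.
; BeginPlay saves the start position and launches the sphere along its right vector with random yaw at constant Speed.
; Hits reflect the direction off the surface normal with slight random yaw.
; Overlapping TriggerP1 scores for P2, any other overlap for P1, then the ball stops, resets and relaunches after delays through Sacar.
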(event Custom|Sacar
  (bind _returnvalue (Math|Random|RandomFloatinRange 5.0 3e+01))
  (bind _sphere (Variables|Default|GetSphere))
  (bind _returnvalue_2 (Math|Vector|GetRightVector _sphere))
  (bind _returnvalue_3 (Math|Vector|RotateVector _returnvalue_2 (Math|Rotator|MakeRotator 0.0 0.0 _returnvalue)))
  ;[1 1 1] Sistema de movimiento base
  (Variables|Default|SetBase%20Position (Transformation|GetActorLocation self))
  ;;[1 1 1] Initial Direction Set
  (Variables|Default|SetCurrent%20Direction _returnvalue_3) ; Set Initial movement Direction
  (Physics|SetPhysicsLinearVelocity (Variables|Default|GetSphere) (* _returnvalue_3 (Variables|Default|GetSpeed)) false "None")
  (bind _outactors (Actor|GetAllActorsOfClass "/Game/Blueprints/PongPlayerController.PongPlayerController_C")))

(event Collision|EventActorBeginOverlap
  (params (OtherActor :type Actor%20Object%20Reference))
  ;[1 1 1] Puntuacion
  ;;[1 1 1] If Actor overlap with TriggerBox
  ;;[1 1 1] Condition Check + Score Up
  (if (== OtherActor (Variables|Default|GetTrigger_P1))
    (Math|Integer|IncrementInt (Variables|Default|Getcounter_P2)
      (:%20%20
        _))
    (else
      (Math|Integer|IncrementInt (Variables|Default|Getcounter_P1)
        (:%20%20
          _))))
  ;;[1 1 1] Stop Velocity
  (Physics|SetPhysicsLinearVelocity (Variables|Default|GetSphere) "0, 0, 0" false "None")
  (Utilities|FlowControl|Delay 0.2)
  ;;[1 1 1] Respawn on Editor location
  (Transformation|SetWorldLocation (Variables|Default|GetSphere) (Variables|Default|GetBase%20Position) false false)
  ;;[1 1 1] Throw from Editor location
  (Utilities|FlowControl|Delay 1.0) ; So it lets time for stuff to happen per goal
  (CallFunction|Sacar))

(event EventTick
  (params (DeltaSeconds :type Float%20%28single-precision%29)))

(event EventBeginPlay
  (bind _returnvalue (Math|Random|RandomFloatinRange 5.0 3e+01))
  (bind _sphere (Variables|Default|GetSphere))
  (bind _returnvalue_2 (Math|Vector|GetRightVector _sphere))
  (bind _returnvalue_3 (Math|Vector|RotateVector _returnvalue_2 (Math|Rotator|MakeRotator 0.0 0.0 _returnvalue)))
  ;[1 1 1] Sistema de movimiento base
  (Variables|Default|SetBase%20Position (Transformation|GetActorLocation self))
  ;;[1 1 1] Initial Direction Set
  (Variables|Default|SetCurrent%20Direction _returnvalue_3) ; Set Initial movement Direction
  (Physics|SetPhysicsLinearVelocity (Variables|Default|GetSphere) (* _returnvalue_3 (Variables|Default|GetSpeed)) false "None")
  (bind _outactors (Actor|GetAllActorsOfClass "/Game/Blueprints/PongPlayerController.PongPlayerController_C")))

(event Collision|EventHit
  (params (MyComp :type Primitive%20Component%20Object%20Reference) (Other :type Actor%20Object%20Reference) (OtherComp :type Primitive%20Component%20Object%20Reference) (bSelfMoved :type Boolean) (HitLocation :type Vector :default "0, 0, 0") (HitNormal :type Vector :default "0, 0, 0") (NormalImpulse :type Vector :default "0, 0, 0") (Hit :type Hit%20Result%20Structure%20%28by%20ref%29))
  ;[1 1 1] Sistema de Rebote
  ;;[1 1 1] On Hit
  ;;[1 1 1] Set Bounce direction
  (bind _output_get (Variables|Default|SetCurrent%20Direction (Math|Vector|RotateVector (Math|Vector|Normalize (Math|Vector|GetReflectionVector (Variables|Default|GetCurrent%20Direction) HitNormal)) (Math|Rotator|MakeRotator 0.0 0.0 (Math|Random|RandomFloatinRange -5.0 5.0)))))
  (Physics|SetPhysicsLinearVelocity (Variables|Default|GetSphere) (* _output_get (Variables|Default|GetSpeed)) false "None"))

(fn ConstructionScript)