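; Desplazador is an actor that the player slides along a straight line between two reference actors, Top and Bottom, using the Vertical input axis.
; BeginPlay enables input from player 0, and each axis event adds speed- and delta-scaled input to a normalized, clamped position.
; That position drives a linear Ease between both actors' locations to set this actor's location without sweep.
; An acceleration timeline for forward movement remains unconnected.
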(event EventBeginPlay
  ;[1 1 1] Se habilita la entrada
  (Input|EnableInput (Game|GetPlayerController 0)))

(event Collision|EventActorBeginOverlap
  (params (OtherActor :type Actor%20Object%20Reference)))

(event EventTick
  (params (DeltaSeconds :type Float%20%28single-precision%29)))

(event Input|AxisEvents|InputAxisVertical
  (params (AxisValue :type Float%20%28single-precision%29)))

(event Input|AxisEvents|InputAxisVertical
  (params (AxisValue :type Float%20%28single-precision%29))
  ;[1 1 1] Control de entrada
  ;[1 1 1] Interpolación de movimiento
  (bind _output_get (Variables|Default|SetPostion (Math|Float|Clamp(Float) (+ (* AxisValue (Variables|Default|GetSpeed) (Utilities|Time|GetWorldDeltaSeconds)) (Variables|Default|GetPostion)))))
  (Transformation|SetActorLocation (Math|Interpolation|Ease "Linear" _output_get (Transformation|GetActorLocation (Variables|Default|GetTop)) (Transformation|GetActorLocation (Variables|Default|GetBottom))) false false))

(fn ConstructionScript)